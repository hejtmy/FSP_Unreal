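; BP_FSPPawn is a pawn that gives the player an on-screen control UI for its CineCamera.
; On BeginPlay it creates a WBP_CameraControls widget, passes it the CineCamera, stores it as CameraUI and shows the mouse cursor on player controller 0.
; ShowCameraControls and HideCameraControls add that widget to the viewport or remove it, and BeginPlay shows it immediately.
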(event `self.ReceiveBeginPlay`
  ;[1 1 1] Adds UI
  (bind _returnvalue (`|CreateWidget` "/FSP/Blueprints/UI/WBP_CameraControls.WBP_CameraControls_C"))
  (set `/FSP/Blueprints/UI/WBP_CameraControls.camera` (`self.CineCamera`) _returnvalue)
  (set `self.CameraUI` _returnvalue)
  (set `PlayerController.bShowMouseCursor` true (`GameplayStatics.GetPlayerController` 0))
  (`self.ShowCameraControls`))

(fn `HideCameraControls`
  (`Widget.RemoveFromParent` (`self.CameraUI`))
  (return))

(fn `ShowCameraControls`
  (`UserWidget.AddToViewport` (`self.CameraUI`) 0)
  (return))

(fn `UserConstructionScript`)