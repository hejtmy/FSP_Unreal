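; BP_DebugHelper is a debug Blueprint that binds hotkeys for testing object transformations and scene analysis.
; H iterates every entry in the ObjectsManager map, resetting objects whose transformation state has changed and changing the state of the rest.
; A runs the CppRecorder's SceneAnalyzer for the first player controller with hit drawing enabled, then prints each key and integer value of the returned map.
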(event `Key|H`
  (params (Key :type "Key Structure"))
  (bind _objects (`FSPObjectManager.Objects` (`self.ObjectsManager`)))
  (:`Pressed`
    (bind _keys (`BlueprintMapLibrary.Map_Keys` _objects))
    (for _array_element _keys
      (bind _value (`BlueprintMapLibrary.Map_Find` _objects _array_element))
      (if (`FSPObject.bTransformationStateChanged` _value)
        (`FSPObject.ResetState` _value)
        (else
          (`FSPObject.ChangeState` _value))))))

(event `Key|A`
  (params (Key :type "Key Structure"))
  (:`Pressed`
    (bind _returnvalue (`FSPSceneAnalyzer.AnalyzeScene` (`FSPRecorder.SceneAnalyzer` (`self.cppRecorder`)) (`GameplayStatics.GetPlayerController` 0) 50 true false))
    (bind _keys (`BlueprintMapLibrary.Map_Keys` _returnvalue))
    (for _array_element _keys
      (`KismetSystemLibrary.PrintString` (`KismetStringLibrary.BuildString_Int` "" (`KismetStringLibrary.Conv_NameToString` _array_element) (`BlueprintMapLibrary.Map_Find` _returnvalue _array_element))))))

(fn `UserConstructionScript`)