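; BP_FSPObjectsManager is a registry that tracks objects by name and moves them on request.
; AddObject stores each object in the Objects map under its Name, or prints a warning and skips it when that key already exists.
; GetObject looks up an object by name, and MoveObject uses that lookup to call Move with a target location if the result is valid.
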(event `self.ReceiveBeginPlay`)

(fn `AddObject`
  (params (Object :type "/FSP/Blueprints/Objects/BP_FSPObjectComponent Object Reference"))
  (bind _name (`/FSP/Blueprints/Objects/BP_FSPObjectComponent.Name` Object))
  ;[1 1 1] Check Key exists
  (if (`BlueprintMapLibrary.Map_Contains` (`self.Objects`) _name)
    ;[1 1 1] Key exits
    (`KismetSystemLibrary.PrintString` (`KismetStringLibrary.BuildString_Name` (`KismetSystemLibrary.GetObjectName` (`ActorComponent.GetOwner` Object)) (`KismetStringLibrary.BuildString_Name` " " "Key " _name " already exits on object  ") "None" "Not creating") true true (struct :`G` 0.66 :`B` 1.0 :`A` 1.0) 5.0)
    (else
      ;[1 1 1] Assigning to Objects
      (`BlueprintMapLibrary.Map_Add` (`self.Objects`) _name Object))))

(fn `GetObject`
  (params (Name :type Name))
  (returns (Value :type "/FSP/Blueprints/Objects/BP_FSPObjectComponent Object Reference"))
  (return (`BlueprintMapLibrary.Map_Find` (`self.Objects`) Name)))

(fn `MoveObject`
  (params (Name :type Name) (Location :type "Vector Structure"))
  (bind _value (`self.GetObject` Name))
  (if (`KismetSystemLibrary.IsValid` _value)
    (`/FSP/Blueprints/Objects/BP_FSPObjectComponent.Move` _value Location)))

(fn `UserConstructionScript`)