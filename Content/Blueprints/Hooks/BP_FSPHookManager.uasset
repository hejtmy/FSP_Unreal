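; Manager for BP_FSPHook camera hooks that cycles the player's view between them and takes high-resolution screenshots.
; On BeginPlay it caches every hook in the level, then steps through them with a wrapping index, switching the first player controller's view target to the selected hook.
; It also exposes the active hook, detaches the view back to the controller, and captures screenshots through the HighResShot console command.
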(event `self.ReceiveBeginPlay`
  ;[1 1 1] Gets all camera hooks
  (bind _outactors (`GameplayStatics.GetAllActorsOfClass` "/FSP/Blueprints/Hooks/BP_FSPHook.BP_FSPHook_C"))
  (bind _output_get (set `self.Hooks` _outactors))
  (set `self.nHooks` (`KismetArrayLibrary.Array_Length` _output_get)))

(event `ActiveScreenshot`
  (`KismetSystemLibrary.ExecuteConsoleCommand` "HighResShot 2" null))

(fn `Detach`
  (bind _returnvalue (`GameplayStatics.GetPlayerController` 0))
  (`PlayerController.SetViewTargetWithBlend` _returnvalue _returnvalue 0.0 "VTBlend_Linear" 0.0 false))

(fn `GetActiveHook`
  (returns (Output :type "/FSP/Blueprints/Hooks/BP_FSPHook Object Reference"))
  (return (`|GetArrayItem` (`self.Hooks`) (`self.iHook`))))

(fn `IncrementHook`
  (locals (iTemp :type Integer))
  (bind _output_get (set `local.iTemp` (+ (`self.iHook`) 1)))
  (if (>= _output_get (`self.nHooks`))
    (set `self.iHook` 0)
    (else
      (set `self.iHook` (`local.iTemp`)))))

(fn `SetNextView`
  (`self.IncrementHook`)
  (`self.SetView` (`self.iHook`)))

(fn `SetView`
  (params (iHook :type Integer))
  (`PlayerController.SetViewTargetWithBlend` (`GameplayStatics.GetPlayerController` 0) (`|GetArrayItem` (`self.Hooks`) iHook) 0.0 "VTBlend_Linear" 0.0 false))

(fn `TakeScreenshot`
  (`KismetSystemLibrary.ExecuteConsoleCommand` "HighResShot 2" null))

(fn `UserConstructionScript`)