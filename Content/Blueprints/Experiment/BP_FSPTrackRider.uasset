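; BP_FSPTrackRider is an actor that rides along the spline of a CameraTrack, apparently as a camera rider, and shows a WBP_TrackControls widget on BeginPlay.
; While moving, Tick advances a normalized TrackPosition over Duration seconds, loops it back to zero, and sets location and rotation from the spline distance.
; Start, stop and switch events toggle movement.
; An alternative Movement timeline path is left unconnected.
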(event `self.ReceiveBeginPlay`
  (bind _returnvalue (`|CreateWidget` "/FSP/Blueprints/UI/WBP_TrackControls.WBP_TrackControls_C"))
  (bind _output_get (set `self.UI` _returnvalue))
  (`UserWidget.AddToViewport` _output_get 0))

(event `SwitchMoving`
  (set `self.isMoving` (not (`self.isMoving`))))

(event `StopMoving`
  (set `self.isMoving` false))

(event `self.ReceiveTick`
  (params (DeltaSeconds :type "Float (single-precision)"))
  (if (`self.isMoving`)
    (if (> (`self.TrackPosition`) 1.0)
      (set `self.TrackPosition` 0.0)
      (else
        (bind _output_get (set `self.TrackPosition` (+ (/ DeltaSeconds (`self.Duration`)) (`self.TrackPosition`))))))
    (`self.SetTrackPosition` _output_get)))

(event `StartMoving`
  (set `self.isMoving` true))

(fn `GetSplinePosition`
  (params (Ratio :type "Float (double-precision)"))
  (returns (Location :type "Vector Structure"))
  (bind _track (`/FSP/Blueprints/Experiment/BP_FSPCameraTrack.Track` (`self.CameraTrack`)))
  (return (`SplineComponent.GetLocationAtDistanceAlongSpline` _track (`KismetMathLibrary.Lerp` 0.0 (`SplineComponent.GetSplineLength` _track) Ratio) "World")))

(fn `GetSplineRotation`
  (params (Ratio :type "Float (double-precision)"))
  (returns (Rotation :type "Rotator Structure"))
  (bind _track (`/FSP/Blueprints/Experiment/BP_FSPCameraTrack.Track` (`self.CameraTrack`)))
  (return (`SplineComponent.GetRotationAtDistanceAlongSpline` _track (`KismetMathLibrary.Lerp` 0.0 (`SplineComponent.GetSplineLength` _track) Ratio) "World")))

(fn `SetTrackPosition`
  (params (Ratio :type "Float (double-precision)"))
  (`self.K2_SetActorLocationAndRotation` (`self.GetSplinePosition` Ratio) (`self.GetSplineRotation` Ratio)))

(fn `UserConstructionScript`)