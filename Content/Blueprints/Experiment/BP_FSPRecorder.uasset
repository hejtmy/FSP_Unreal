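; BP_FSPRecorder captures a series of high-resolution screenshots at evenly spaced positions along the controller's track rider component.
; StartScreenshotting runs a macro that stops the rider, hides its controls, then uses a delayed loop to reposition it and fire HighResShot.
; It broadcasts each shot and completion, restoring movement and controls at the end.
; A separate CreateScreenshots function does a similar capture without delays and is not called here.
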(event `StartScreenshotting`
  (`self.Screenshotting`
    (:`out`
      (`self.ScreenshotsFinished`))))

(fn `CreateScreenshots`
  (params (nScreenshots :type Integer))
  (locals (ScreenshotOffset :type "Float (double-precision)"))
  (bind _bp_fsptrackridercomponent (`/FSP/Blueprints/Controller/BP_FSPPawn.BP_FSPTrackRiderComponent` (`self.Controller`)))
  (`/FSP/Blueprints/Experiment/BP_FSPTrackRiderComponent.HideControls` _bp_fsptrackridercomponent)
  (bind _output_get (set `local.ScreenshotOffset` (/ 1.0 (`KismetMathLibrary.Conv_IntToDouble` (- nScreenshots 1)))))
  (for _index (range (+ nScreenshots 1))
    (`/FSP/Blueprints/Experiment/BP_FSPTrackRiderComponent.SetTrackPosition` _bp_fsptrackridercomponent (* _index _output_get))
    (`KismetSystemLibrary.ExecuteConsoleCommand` "HighResShot 1920x1080" null))
  (`/FSP/Blueprints/Experiment/BP_FSPTrackRiderComponent.ShowControls` _bp_fsptrackridercomponent)
  (return))

(fn `UserConstructionScript`)