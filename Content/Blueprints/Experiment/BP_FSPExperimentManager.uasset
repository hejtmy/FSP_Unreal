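; BP_FSPExperimentManager is a debug-style controller that maps keyboard keys to experiment actions.
; On BeginPlay it finds the hook manager and objects manager actors if unset, and takes the recorder component from the controller.
; Keys cycle hook views, take screenshots, detach the hook, move a hardcoded test object to the origin, toggle recording, and quit the game.
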(event `self.ReceiveBeginPlay`
  (`/Engine/EditorBlueprintResources/StandardMacros.IsValid` (`self.HookManager`)
    (:`Is Valid`
      _)
    (:`Is Not Valid`
      (bind _returnvalue (`GameplayStatics.GetActorOfClass` "/FSP/Blueprints/Hooks/BP_FSPHookManager.BP_FSPHookManager_C"))
      (set `self.HookManager` _returnvalue)))
  (`/Engine/EditorBlueprintResources/StandardMacros.IsValid` (`self.ObjectManager`)
    (:`Is Valid`
      _)
    (:`Is Not Valid`
      (bind _returnvalue_2 (`GameplayStatics.GetActorOfClass` "/FSP/Blueprints/Objects/BP_FSPObjectsManager.BP_FSPObjectsManager_C"))
      (set `self.ObjectManager` _returnvalue_2)))
  (set `self.Recorder` (`self.GetComponentByClass` (`self.Controller`) "/FSP/Blueprints/Experiment/BP_FSPRecorder.BP_FSPRecorder_C")))

(event `Key|C`
  (params (Key :type "Key Structure"))
  (:`Pressed`
    (`/FSP/Blueprints/Hooks/BP_FSPHookManager.SetNextView` (`self.HookManager`))))

(event `Key|P`
  (params (Key :type "Key Structure"))
  (:`Pressed`
    (`/FSP/Blueprints/Hooks/BP_FSPHookManager.TakeScreenshot` (`self.HookManager`))))

(event `Key|M`
  (params (Key :type "Key Structure"))
  (:`Pressed`
    (`/FSP/Blueprints/Objects/BP_FSPObjectsManager.MoveObject` (`self.ObjectManager`) "Object2" (0.0 0.0 0.0))))

(event `Key|O`
  (params (Key :type "Key Structure"))
  (:`Pressed`
    (`/FSP/Blueprints/Hooks/BP_FSPHookManager.Detach` (`self.HookManager`))))

(event `Key|Escape`
  (params (Key :type "Key Structure"))
  (:`Pressed`
    (`KismetSystemLibrary.QuitGame` null "Quit")))

(event `Key|R`
  (params (Key :type "Key Structure"))
  (:`Pressed`
    (`/FSP/Blueprints/Experiment/BP_FSPRecorder.SwitchRecording` (`self.Recorder`))))

(fn `UserConstructionScript`)