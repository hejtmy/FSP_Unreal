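; Actor component that moves and rotates its owner along the spline of a referenced CameraTrack.
; While IsMoving, Tick places the owner at the normalized TrackPosition, sampled by spline distance in world space.
; With MoveAutomatically on, the position advances over Duration, then signals track end and wraps to the start.
; Start, stop and switch events control automatic movement; show/hide functions expect a UI widget, whose creation code is disconnected.
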(event `self.ReceiveBeginPlay`)

(event `SwitchMoving`
  ;[1 1 1] Turhing things on and off
  (set `self.moveAutomatically` (not (`self.moveAutomatically`))))

(event `self.ReceiveTick`
  (params (DeltaSeconds :type "Float (single-precision)"))
  (if (`self.isMoving`)
    (`self.SetTrackPosition` (`self.TrackPosition`))
    (if (`self.moveAutomatically`)
      (`self.UpdateTrackPosition` DeltaSeconds))))

(event `StartMoving`
  ;[1 1 1] Turhing things on and off
  (set `self.moveAutomatically` true))

(event `StopMoving`
  ;[1 1 1] Turhing things on and off
  (set `self.moveAutomatically` false))

(fn `GetSplinePosition`
  (params (ratio :type "Float (double-precision)"))
  (returns (Location :type "Vector Structure"))
  (bind _cameratrack (`/FSP/Blueprints/Experiment/BP_FSPCameraTrack.CameraTrack` (`self.CameraTrack`)))
  (return (`SplineComponent.GetLocationAtDistanceAlongSpline` _cameratrack (`KismetMathLibrary.Lerp` 0.0 (`SplineComponent.GetSplineLength` _cameratrack) ratio) "World")))

(fn `GetSplineRotation`
  (params (ratio :type "Float (double-precision)"))
  (returns (Rotation :type "Rotator Structure"))
  (bind _cameratrack (`/FSP/Blueprints/Experiment/BP_FSPCameraTrack.CameraTrack` (`self.CameraTrack`)))
  (return (`SplineComponent.GetRotationAtDistanceAlongSpline` _cameratrack (`KismetMathLibrary.Lerp` 0.0 (`SplineComponent.GetSplineLength` _cameratrack) ratio) "World")))

(fn `HideControls`
  (`Widget.RemoveFromParent` (`self.UI`))
  (return))

(fn `SetTrackPosition`
  (params (ratio :type "Float (double-precision)"))
  (set `self.TrackPosition` ratio)
  (`Actor.K2_SetActorLocationAndRotation` (`self.GetOwner`) (`self.GetSplinePosition` ratio) (`self.GetSplineRotation` ratio) false false))

(fn `ShowControls`
  (`UserWidget.AddToViewport` (`self.UI`) 0)
  (return))

(fn `UpdateTrackPosition`
  (params (delta :type "Float (double-precision)"))
  (if (> (`self.TrackPosition`) 1.0)
    (`self.TrackEndReached`)
    (set `self.TrackPosition` 0.0)
    (else
      (set `self.TrackPosition` (+ (/ delta (`self.Duration`)) (`self.TrackPosition`)))))
  (return))